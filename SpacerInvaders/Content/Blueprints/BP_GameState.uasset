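; Game state for a wave-based enemy shooter, holding score, player HP, level, enemy count and shared enemy stats.
; Helper functions update score, HP and enemy count, flagging game over at zero HP, while a separate event calls GameOver on the player controller.
; WaveCleared, when no enemies remain, has the wave manager spawn a wave, then raises the level, compounding enemy stats by percentages.
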(event Custom|WaveCleared
  ;[1 1 1] Sekwencja konca fali
  (if (< (Variables|Default|GetNumberOfEnemies) 1)
    (bind _outactors (Actor|GetAllActorsOfClass "/Game/Blueprints/BP_WaveManager.BP_WaveManager_C"))
    (Default|SpawnWave (Utilities|Array|Get(acopy) _outactors))
    (CallFunction|IncreaseLevel)))

(event Custom|TriggerGameOver
  ;[1 1 1] Sekwencja konca gry
  (bind _asbp_player_controller (Utilities|Casting|CastToBP_PlayerController (Game|GetPlayerController 0)))
  (Default|GameOver _asbp_player_controller))

(fn ConstructionScript)

(fn AddScore
  (params (Amount :type Integer))
  (Variables|Default|SetScore (+ Amount (Variables|Default|GetScore))))

(fn DealDamage
  (params (Amount :type Integer))
  (Variables|Default|SetPlayerHP (- (Variables|Default|GetPlayerHP) Amount))
  (if (<= (Variables|Default|GetPlayerHP) 0)
    (Variables|Default|SetbGameOver true)))

(fn DecreaseEnemyNumber
  (Variables|Default|SetNumberOfEnemies (- (Variables|Default|GetNumberOfEnemies) 1)))

(fn IncreaseLevel
  (Variables|Default|SetLevel (+ (Variables|Default|GetLevel) 1))
  (bind _output_get (Variables|Default|SetStats (Utilities|Struct|MakeS_ActorsStats (+ (* (.enemy_shotchance (Variables|Default|GetStats)) 0.2) (.enemy_shotchance (Variables|Default|GetStats))) (Math|Vector|MakeVector (- (.x (.enemy_shottimerange (Variables|Default|GetStats))) (* (.x (.enemy_shottimerange (Variables|Default|GetStats))) 0.1)) (- (.y (.enemy_shottimerange (Variables|Default|GetStats))) (* (.y (.enemy_shottimerange (Variables|Default|GetStats))) 0.1)) 0.0) (+ (* (.enemy_bulletspeed (Variables|Default|GetStats)) 0.25) (.enemy_bulletspeed (Variables|Default|GetStats))) (+ (* (.enemy_movingfrequency (Variables|Default|GetStats)) 0.1) (.enemy_movingfrequency (Variables|Default|GetStats))) (+ (* (.enemy_fallspeed (Variables|Default|GetStats)) 0.9) (.enemy_fallspeed (Variables|Default|GetStats)))))))