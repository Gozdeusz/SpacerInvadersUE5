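; Enemy ship actor for a wave-based shooter, with three types that set mesh, material and score value.
; Tick moves it in a sine sway along X, flipped by Side, while descending on Z, using speeds from GameState stats.
; A looping timer, with an interval randomized once at BeginPlay, fires bullets by chance.
; Destruction updates GameState enemy count, wave check and score, then spawns a score popup.
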(event Custom|Shoot
  ;[1 1 1] Strzelanie
  ;;[0.1854 0.1728 1] Szansa na oddanie strzału
  (bind _asbp_game_state (Utilities|Casting|CastToBP_GameState (Game|GetGameState)))
  (if (< (Math|Random|RandomFloatinRange 0.0 1.0) (Utilities|Struct|BreakS_ActorsStats (Variables|/Game/Blueprints/BP_GameState.BP_GameState_C|GetStats _asbp_game_state)))
    (Game|SpawnActorfromClass "/Game/Blueprints/BP_Enemy_Bullet.BP_Enemy_Bullet_C" (Math|Conversions|ToTransform(Vector) (Transformation|GetWorldLocation (Variables|Default|GetShootingPoint))) "Undefined" "MultiplyWithRoot" 0 0)))

(event EventBeginPlay
  ;[1 1 1] Ustawienie zmiennej okreslajacej pozycje i czasu strzelania
  (bind _asbp_game_state (Utilities|Casting|CastToBP_GameState (Game|GetGameState)))
  (CallFunction|SwitchModel (Variables|Default|GetEnemyType))
  (Variables|Default|SetElapsed%20Time 0.0)
  (Variables|Default|SetFrequency (.Enemy_MovingFrequency (Utilities|Struct|BreakS_ActorsStats (Variables|/Game/Blueprints/BP_GameState.BP_GameState_C|GetStats _asbp_game_state))))
  (Variables|Default|SetMoveSpeed (.Enemy_FallSpeed (Utilities|Struct|BreakS_ActorsStats (Variables|/Game/Blueprints/BP_GameState.BP_GameState_C|GetStats _asbp_game_state))))
  (Variables|Default|SetStartLocation (Transformation|GetActorLocation))
  (Utilities|Time|SetTimerbyFunctionName 0 "Shoot" (Math|Random|RandomFloatinRange (.X (Math|Vector|BreakVector (.Enemy_ShotTimeRange (Utilities|Struct|BreakS_ActorsStats (Variables|/Game/Blueprints/BP_GameState.BP_GameState_C|GetStats _asbp_game_state))))) (.Y (Math|Vector|BreakVector (.Enemy_ShotTimeRange (Utilities|Struct|BreakS_ActorsStats (Variables|/Game/Blueprints/BP_GameState.BP_GameState_C|GetStats _asbp_game_state)))))) true))

(event EventTick
  (params (DeltaSeconds :type Float%20%28single-precision%29))
  (bind _startlocation (Variables|Default|GetStartLocation))
  ;[1 1 1] Ruch
  (Variables|Default|SetElapsed%20Time (+ DeltaSeconds (Variables|Default|GetElapsed%20Time)))
  (Transformation|SetActorLocation (Math|Vector|MakeVector (* (+ (* (Math|Trig|Sin(Radians) (* (Utilities|Time|GetGameTimeinSeconds) (Variables|Default|GetFrequency))) (Variables|Default|GetAmplitude)) (.x _startlocation)) (Variables|Default|GetSide)) (.y _startlocation) (+ (.z _startlocation) (* (Variables|Default|GetElapsed%20Time) (Variables|Default|GetMoveSpeed) -1.0))) false false))

(event EventDestroyed
  (bind _scoreamount (Variables|Default|GetScoreAmount))
  ;[1 1 1] Funkcje wykonane po zniszczeniu przeciwnika
  (bind _asbp_game_state (Utilities|Casting|CastToBP_GameState (Game|GetGameState)))
  (Default|DecreaseEnemyNumber _asbp_game_state)
  (Default|WaveCleared _asbp_game_state)
  (Default|AddScore _asbp_game_state _scoreamount)
  (Game|SpawnActorfromClass "/Game/Blueprints/BP_ScoreText.BP_ScoreText_C" (Math|Conversions|ToTransform(Vector) (Transformation|GetActorLocation)) "Undefined" "MultiplyWithRoot" 0 _scoreamount 0))

(fn ConstructionScript)

(fn SwitchModel
  (params (Number :type Integer))
  (switch int Number
    (:1
      (Variables|Default|SetEnemyMesh "/Game/Fab/StarSparrow/Meshes/Examples/SM_StarSparrow02.SM_StarSparrow02")
      (Variables|Default|SetMeshMaterial "/Game/Fab/StarSparrow/Materials/M_StarSparrow_Blue.M_StarSparrow_Blue")
      (Variables|Default|SetScoreAmount 100))
    (:2
      (Variables|Default|SetEnemyMesh "/Game/Fab/StarSparrow/Meshes/Examples/SM_StarSparrow05.SM_StarSparrow05")
      (Variables|Default|SetMeshMaterial "/Game/Fab/StarSparrow/Materials/M_StarSparrow_Green.M_StarSparrow_Green")
      (Variables|Default|SetScoreAmount 200))
    (:3
      (Variables|Default|SetEnemyMesh "/Game/Fab/StarSparrow/Meshes/Examples/SM_StarSparrow09.SM_StarSparrow09")
      (Variables|Default|SetMeshMaterial "/Game/Fab/StarSparrow/Materials/M_StarSparrow_White.M_StarSparrow_White")
      (Variables|Default|SetScoreAmount 500)))
  (Components|StaticMesh|SetStaticMesh (Variables|Default|GetEnemyModelMesh) (Variables|Default|GetEnemyMesh))
  (Rendering|Material|SetMaterial (Variables|Default|GetEnemyModelMesh) 0 (Variables|Default|GetMeshMaterial)))