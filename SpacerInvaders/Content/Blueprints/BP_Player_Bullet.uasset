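; BP_Player_Bullet is the player's projectile, which destroys enemies on contact.
; Each tick it moves along its local Z axis by Speed scaled by delta time, and destroys itself once its world Z passes a fixed limit.
; When its Collision component overlaps a BP_Enemy, it destroys both the enemy and itself, ignoring all other actors.
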(event OnComponentBeginOverlap(Collision)
  (params (OverlappedComponent :type Primitive%20Component%20Object%20Reference) (OtherActor :type Actor%20Object%20Reference) (OtherComp :type Primitive%20Component%20Object%20Reference) (OtherBodyIndex :type Integer) (bFromSweep :type Boolean) (SweepResult :type Hit%20Result%20Structure%20%28by%20ref%29))
  ;[1 1 1] Zdarzenie pocisku z przeciwnikiem
  (bind _asbp_enemy (Utilities|Casting|CastToBP_Enemy OtherActor))
  (Actor|DestroyActor _asbp_enemy)
  (Actor|DestroyActor))

(event EventTick
  (params (DeltaSeconds :type Float%20%28single-precision%29))
  ;[1 1 1] Ruch pocisku
  (Transformation|AddActorLocalOffset (Math|Vector|MakeVector 0.0 0.0 (* (Variables|Default|GetSpeed) (Utilities|Time|GetWorldDeltaSeconds))) false false)
  ;[1 1 1] Zniszczenie pocisku po osiagnieciu pozycji
  (if (> (.z (Transformation|GetActorLocation)) 1e+04)
    (Actor|DestroyActor)))

(fn ConstructionScript)