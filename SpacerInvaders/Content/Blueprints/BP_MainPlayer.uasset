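; Player pawn for a shooter: slides sideways on input within a clamped range and fires bullets from a shot point after a short delay.
; Movement offsets local Y, then clamps world X to MovementRange.
; Enemy bullets overlapping either collider deal damage through BP_GameState, triggering game over or temporary invulnerability.
; That window disables collision while a timeline flickers the mesh and drives a material-parameter effect, alongside camera shake.
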(event OnComponentBeginOverlap(PlayerCollision)
  (params (OverlappedComponent :type Primitive%20Component%20Object%20Reference) (OtherActor :type Actor%20Object%20Reference) (OtherComp :type Primitive%20Component%20Object%20Reference) (OtherBodyIndex :type Integer) (bFromSweep :type Boolean) (SweepResult :type Hit%20Result%20Structure%20%28by%20ref%29))
  (bind _playercollision (Variables|Default|GetPlayerCollision))
  (bind _player_collision_2 (Variables|Default|GetPlayer%20Collision%202))
  ;[1 1 1] Otrzymanie obrazen
  (Utilities|Casting|CastToBP_Enemy_Bullet OtherActor)
  (bind _asbp_game_state (Utilities|Casting|CastToBP_GameState (Game|GetGameState)))
  (Default|DealDamage _asbp_game_state 1)
  (if (< (Variables|/Game/Blueprints/BP_GameState.BP_GameState_C|GetPlayerHP _asbp_game_state) 1)
    (Default|TriggerGameOver _asbp_game_state)
    (else
      ;;[0 0.4969 0.6038] Efekt otrzymania obrazen i wylaczenie kolizji
      (Collision|SetCollisionEnabled _playercollision "NoCollision")
      (Collision|SetCollisionEnabled _player_collision_2 "NoCollision")
      (CameraShakes|StartCameraShake (Game|GetPlayerCameraManager 0) "/Game/Blueprints/CS_DamageShake.CS_DamageShake_C" 1.0 "CameraLocal" "0, 0, 0")
      (bind _caflow (Timeline|Timeline PlayFromStart)
        (:Update
          (Rendering|Material|SetScalarParameterValue "/Game/EffectsAndShaders/ChromaticAberration/MPC_CA.MPC_CA" "HealthFactor" _caflow :!class /Script/Engine.KismetMaterialLibrary)
          (Utilities|FlowControl|FlipFlop
            (:A
              (Rendering|SetVisibility (Variables|Default|GetPlayerModelMesh) true false))
            (:B
              (Rendering|SetVisibility (Variables|Default|GetPlayerModelMesh) false false))))
        (:Finished
          (Collision|SetCollisionEnabled _playercollision "QueryAndPhysics")
          (Collision|SetCollisionEnabled _player_collision_2 "QueryAndPhysics")
          (Rendering|SetVisibility (Variables|Default|GetPlayerModelMesh) true false))))))

(event OnComponentBeginOverlap(PlayerCollision2)
  (params (OverlappedComponent :type Primitive%20Component%20Object%20Reference) (OtherActor :type Actor%20Object%20Reference) (OtherComp :type Primitive%20Component%20Object%20Reference) (OtherBodyIndex :type Integer) (bFromSweep :type Boolean) (SweepResult :type Hit%20Result%20Structure%20%28by%20ref%29))
  (bind _playercollision (Variables|Default|GetPlayerCollision))
  (bind _player_collision_2 (Variables|Default|GetPlayer%20Collision%202))
  ;[1 1 1] Otrzymanie obrazen
  (Utilities|Casting|CastToBP_Enemy_Bullet OtherActor)
  (bind _asbp_game_state (Utilities|Casting|CastToBP_GameState (Game|GetGameState)))
  (Default|DealDamage _asbp_game_state 1)
  (if (< (Variables|/Game/Blueprints/BP_GameState.BP_GameState_C|GetPlayerHP _asbp_game_state) 1)
    (Default|TriggerGameOver _asbp_game_state)
    (else
      ;;[0 0.4969 0.6038] Efekt otrzymania obrazen i wylaczenie kolizji
      (Collision|SetCollisionEnabled _playercollision "NoCollision")
      (Collision|SetCollisionEnabled _player_collision_2 "NoCollision")
      (CameraShakes|StartCameraShake (Game|GetPlayerCameraManager 0) "/Game/Blueprints/CS_DamageShake.CS_DamageShake_C" 1.0 "CameraLocal" "0, 0, 0")
      (bind _caflow (Timeline|Timeline PlayFromStart)
        (:Update
          (Rendering|Material|SetScalarParameterValue "/Game/EffectsAndShaders/ChromaticAberration/MPC_CA.MPC_CA" "HealthFactor" _caflow :!class /Script/Engine.KismetMaterialLibrary)
          (Utilities|FlowControl|FlipFlop
            (:A
              (Rendering|SetVisibility (Variables|Default|GetPlayerModelMesh) true false))
            (:B
              (Rendering|SetVisibility (Variables|Default|GetPlayerModelMesh) false false))))
        (:Finished
          (Collision|SetCollisionEnabled _playercollision "QueryAndPhysics")
          (Collision|SetCollisionEnabled _player_collision_2 "QueryAndPhysics")
          (Rendering|SetVisibility (Variables|Default|GetPlayerModelMesh) true false))))))

(event Input|ActionEvents|InputActionShooting
  (params (Key :type Key%20Structure :default "None"))
  ;[1 1 1] Strzelanie
  (:Pressed
    (Utilities|FlowControl|Delay 0.2)
    (Game|SpawnActorfromClass "/Game/Blueprints/BP_Player_Bullet.BP_Player_Bullet_C" (Math|Conversions|ToTransform(Vector) (Transformation|GetWorldLocation (Variables|Default|GetPlayerShotPoint))) "Undefined" "MultiplyWithRoot" 0 0)))

(event Input|AxisEvents|InputAxisMoveRight
  (params (AxisValue :type Float%20%28single-precision%29))
  (bind _movementrange (Variables|Default|GetMovementRange))
  ;[1 1 1] Ruch gracza
  (Transformation|AddActorLocalOffset (Math|Vector|MakeVector 0.0 (* AxisValue (Variables|Default|GetSpeed) (Utilities|Time|GetWorldDeltaSeconds)) 0.0) false false)
  ;;[0 0.4969 0.6038] Ograniczenie zasiegu ruchu
  (CallFunction|CharacterMovementRangeRestriction (.x _movementrange) (.y _movementrange)))

(event Input|AxisEvents|InputAxisMoveLeft
  (params (AxisValue :type Float%20%28single-precision%29))
  (bind _movementrange (Variables|Default|GetMovementRange))
  ;[1 1 1] Ruch gracza
  (Transformation|AddActorLocalOffset (Math|Vector|MakeVector 0.0 (* AxisValue (Variables|Default|GetSpeed) (Utilities|Time|GetWorldDeltaSeconds)) 0.0) false false)
  ;;[0 0.4969 0.6038] Ograniczenie zasiegu ruchu
  (CallFunction|CharacterMovementRangeRestriction (.x _movementrange) (.y _movementrange)))

(event Input|KeyboardEvents|DebugKey1
  (params (Key :type Key%20Structure :default "None") (ActionValue :type Input%20Action%20Value%20Structure))
  (bind _returnvalue (Game|GetPlayerController 0))
  ;[1 1 1] Debugowanie - wyjscie na ekran
  (:Pressed
    (Utilities|FlowControl|FlipFlop
      (:A
        (Input|SetInputModeGameandUI _returnvalue 0 "DoNotLock" true false)
        (Variables|/Script/Engine.PlayerController|SetbShowMouseCursor _returnvalue true))
      (:B
        (Input|SetInputModeGameandUI _returnvalue 0 "DoNotLock" true false)
        (Variables|/Script/Engine.PlayerController|SetbShowMouseCursor _returnvalue false)))))

(fn ConstructionScript)

(fn CharacterMovementRangeRestriction
  (params (Min :type Float%20%28double-precision%29) (Max :type Float%20%28double-precision%29))
  (bind _returnvalue (Transformation|GetActorLocation))
  (Transformation|SetActorLocation (Math|Vector|MakeVector (Math|Float|Clamp(Float) (.x _returnvalue) Min Max) (.y _returnvalue) (.z _returnvalue)) false false))