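; BP_Asteroid is an asteroid actor that spins and falls until it is removed.
; On BeginPlay it enables custom depth rendering on its mesh for a toon shader.
; Each tick it pitches the mesh by RotationSpeed and moves the actor down its local Z by FallingSpeed with sweep, both scaled by delta time.
; It destroys itself once it drops below a fixed world height.
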(event EventBeginPlay
  ;[1 1 1] Konfiguracja dla dzialania toonshadera
  (Rendering|SetRenderCustomDepth (Variables|Default|GetAsteroidMesh) true))

(event EventTick
  (params (DeltaSeconds :type Float%20%28single-precision%29))
  ;[1 1 1] Opadanie, wirowanie, zycie aktora
  (Transformation|AddLocalRotation (Variables|Default|GetAsteroidMesh) (Math|Rotator|MakeRotator 0.0 (* DeltaSeconds (Variables|Default|GetRotationSpeed)) 0.0) false false)
  (Transformation|AddActorLocalOffset (Math|Vector|MakeVector 0.0 0.0 (* (Variables|Default|GetFallingSpeed) -1.0 DeltaSeconds)) true false)
  ;;[0.0822 0.05554 0.3781] Usuniecie aktora po osiagnieciu pozycji
  (if (< (.z (Transformation|GetActorLocation)) -2e+03)
    (Actor|DestroyActor)))

(fn ConstructionScript)