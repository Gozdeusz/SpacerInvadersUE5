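; Wave manager actor that spawns a grid of BP_Enemy actors at its own location when play begins.
; SpawnWave, called once BP_GameState is cast and cached, runs SpawnEnemyGrid, which writes the total enemy count to the game state.
; The grid extends along +X and down Z, with each row getting its own EnemyType and an alternating Side value passed to the spawned enemies.
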(event Custom|SpawnWave
  ;[1 1 1] Ustawienia fali
  (Variables|Default|SetStartingLocation (Transformation|GetActorLocation))
  (CallFunction|SpawnEnemyGrid 3 8 3.5e+02))

(event EventBeginPlay
  ;[1 1 1] Spawn fali
  (bind _asbp_game_state (Utilities|Casting|CastToBP_GameState (Game|GetGameState)))
  (Variables|Default|SetGame%20State _asbp_game_state)
  (CallFunction|SpawnWave))

(fn ConstructionScript)

(fn SpawnEnemyGrid
  (params (Rows :type Integer) (Columns :type Integer) (EnemySpacing :type Float%20%28double-precision%29))
  ;[1 1 1] Ustawienie ilosci przeciwnikow dla systemu gry
  (Variables|/Game/Blueprints/BP_GameState.BP_GameState_C|SetNumberOfEnemies (Variables|Default|GetGame%20State) (* Rows Columns))
  ;[1 1 1] Generowanie siatki przeciwnikow i zmiana ich stanu dla kazdego rzedu
  (for _index (range 0 (- Rows 1))
    (CallFunction|SwitchEnemyType _index)
    (bind _sideswitcher (CallFunction|SwitchSide _index))
    (LocalVariables|SetSide _sideswitcher)
    (for _index_2 (range 0 (- Columns 1))
      (bind _output_get (LocalVariables|SetPos (+ (Variables|Default|GetStartingLocation) (Math|Vector|MakeVector (* _index_2 EnemySpacing) 0.0 (* _index EnemySpacing -1.0)))))
      (Game|SpawnActorfromClass "/Game/Blueprints/BP_Enemy.BP_Enemy_C" (Math|Conversions|ToTransform(Vector) _output_get) "Undefined" "MultiplyWithRoot" 0 15.0 (Variables|Default|GetEnemyType) (LocalVariables|GetSide) 0))))

(fn SwitchEnemyType
  (params (Row :type Integer))
  (switch int Row
    (:0
      (Variables|Default|SetEnemyType 3))
    (:1
      (Variables|Default|SetEnemyType 2))
    (:2
      (Variables|Default|SetEnemyType 1))))

(fn SwitchSide
  (params (Row :type Integer))
  (if (== (Math|Integer|%(Integer) Row 2) 0)
    (return 1)
    (else
      (return -1))))