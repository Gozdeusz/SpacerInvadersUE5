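; BP_Enemy_Bullet is an enemy projectile that flies downward and destroys itself when it hits the player.
; Each tick it moves along negative local Z, using EnemyBulletSpeed from the BP_GameState stats scaled by delta time.
; A sphere overlap with BP_MainPlayer destroys the bullet without applying damage here, and a lifespan set on BeginPlay removes stray bullets.
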(event OnComponentBeginOverlap(Sphere)
  (params (OverlappedComponent :type Primitive%20Component%20Object%20Reference) (OtherActor :type Actor%20Object%20Reference) (OtherComp :type Primitive%20Component%20Object%20Reference) (OtherBodyIndex :type Integer) (bFromSweep :type Boolean) (SweepResult :type Hit%20Result%20Structure%20%28by%20ref%29))
  ;[1 1 1] Kolizja pocisku z graczem
  (Utilities|Casting|CastToBP_MainPlayer OtherActor)
  (Actor|DestroyActor))

(event EventBeginPlay
  ;[1 1 1] Czas zycia pocisku
  (Actor|SetLifeSpan 1e+01))

(event EventTick
  (params (DeltaSeconds :type Float%20%28single-precision%29))
  ;[1 1 1] Lot pocisku w dol
  (bind _asbp_game_state (Utilities|Casting|CastToBP_GameState (Game|GetGameState)))
  (Transformation|AddActorLocalOffset (Math|Vector|MakeVector 0.0 0.0 (* (.Enemy_BulletSpeed (Utilities|Struct|BreakS_ActorsStats (Variables|/Game/Blueprints/BP_GameState.BP_GameState_C|GetStats _asbp_game_state))) (Utilities|Time|GetWorldDeltaSeconds) -1.0)) false false))

(fn ConstructionScript)