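; Asteroid spawner actor that creates BP_Asteroid instances on BeginPlay and then repeatedly on a looping timer set by SpawnInterval.
; Each spawn is offset from the spawner's location along world X only, by a random value between SpawnAreaSize.X and SpawnAreaSize.Z, which act as min and max bounds.
; The spawner passes its RotationSpeed and FallingSpeed values to each new asteroid.
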(event EventBeginPlay
  ;[1 1 1] Spawn obiektow
  (CallFunction|SpawnAsteroids)
  (Utilities|Time|SetTimerbyFunctionName 0 "SpawnAsteroids" (Variables|Default|GetSpawnInterval) true))

(fn ConstructionScript)

(fn SpawnAsteroids
  (bind _spawnareasize (Variables|Default|GetSpawnAreaSize))
  (Game|SpawnActorfromClass "/Game/Blueprints/BP_Asteroid.BP_Asteroid_C" (Math|Conversions|ToTransform(Vector) (+ (Transformation|GetActorLocation) (Math|Vector|MakeVector (Math|Random|RandomFloatinRange (.x _spawnareasize) (.z _spawnareasize)) 0.0 0.0))) "Undefined" "MultiplyWithRoot" 0 (Variables|Default|GetRotationSpeed) (Variables|Default|GetFallingSpeed) 0))