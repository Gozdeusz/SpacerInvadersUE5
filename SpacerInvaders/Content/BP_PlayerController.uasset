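; Player controller Blueprint that sets up the HUD and handles restart, quit and game over for the player.
; BeginPlay enables input and adds the WB_HUD widget, while the Restart and Exit input actions reload the level or quit the game.
; The GameOver event shows WB_GameOver with a mouse cursor and UI-only input.
; RestartGame reopens the hard-referenced TestLevelFordevelop level and restores game-only input with the cursor hidden.
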(event Custom|GameOver
  (bind _returnvalue (Game|GetPlayerController 0))
  (bind _returnvalue_2 (UserInterface|CreateWidget "/Game/UI/WB_GameOver.WB_GameOver_C"))
  (UserInterface|Viewport|AddtoViewport _returnvalue_2 0)
  (Variables|/Script/Engine.PlayerController|SetbShowMouseCursor _returnvalue true)
  (Input|SetInputModeUIOnly _returnvalue _returnvalue_2 "DoNotLock" false))

(event EventBeginPlay
  ;[1 1 1] Konfiguracja ustawien
  (Input|EnableInput 0)
  (bind _returnvalue (UserInterface|CreateWidget "/Game/UI/WB_HUD.WB_HUD_C"))
  (UserInterface|Viewport|AddtoViewport _returnvalue 0))

(event Input|ActionEvents|InputActionRestart
  (params (Key :type Key%20Structure :default "None"))
  (:Pressed
    (CallFunction|RestartGame)))

(event Input|ActionEvents|InputActionExit
  (params (Key :type Key%20Structure :default "None"))
  (:Pressed
    (Game|QuitGame 0 "Quit" false)))

(fn ConstructionScript)

(fn RestartGame
  (Game|OpenLevel(byObjectReference) "/Game/Levels/TestLevelFordevelop.TestLevelFordevelop")
  (Input|SetInputModeGameOnly (Game|GetPlayerController 0) false)
  (Variables|Default|SetbShowMouseCursor false))